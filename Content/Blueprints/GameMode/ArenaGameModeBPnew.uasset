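; Arena game mode that sets up the current puzzle level and handles winning and losing.
; BeginPlay switches on the game instance's level to call its setup function and show a delayed hint, with background music alongside; levels 1 and 4 both run Level4, leaving Level1 unwired.
; Win and Loose play sounds and show UI-only result screens.
; Win also saves the fewest moves per level and unlocks the next.
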(event `self.ReceiveBeginPlay`
  (`KismetSystemLibrary.Delay` 2.0)
  (bind _asa_game_instance (cast `/Game/Blueprints/A_GameInstance` (`GameplayStatics.GetGameInstance`)))
  (set `self.As A Game Instance` _asa_game_instance)
  (`|ExecutionSequence`
    (:`then_0`
      (switch `int` (`/Game/Blueprints/A_GameInstance.level` _asa_game_instance)
        (:`1`
          (`self.Level4` :!label _label)
          (`KismetSystemLibrary.Delay` 60.0)
          (bind _returnvalue (`|CreateWidget` "/Game/Blueprints/Hud/W_Hint.W_Hint_C" null "TNT can travel in different dimensions"))
          (`UserWidget.AddToViewport` _returnvalue 0))
        (:`2`
          (`self.Level2`)
          (`KismetSystemLibrary.Delay` 60.0)
          (bind _returnvalue_2 (`|CreateWidget` "/Game/Blueprints/Hud/W_Hint.W_Hint_C" null "Hint - Sometimes enemy is your friend"))
          (`UserWidget.AddToViewport` _returnvalue_2 0))
        (:`3`
          (`self.Level3`)
          (`KismetSystemLibrary.Delay` 60.0)
          (bind _returnvalue_3 (`|CreateWidget` "/Game/Blueprints/Hud/W_Hint.W_Hint_C" null "Hint - Red is really dummy , do you want to change it "))
          (`UserWidget.AddToViewport` _returnvalue_3 0))
        (:`4`
          (goto _label))
        (:`5`
          (`self.Level5`)
          (`KismetSystemLibrary.Delay` 60.0)
          (bind _returnvalue_4 (`|CreateWidget` "/Game/Blueprints/Hud/W_Hint.W_Hint_C" null "Hint - Enenmy's enemy is your friend"))
          (`UserWidget.AddToViewport` _returnvalue_4 0))
        (:`6`
          (`self.Level6`)
          (`KismetSystemLibrary.Delay` 30.0)
          (bind _returnvalue_5 (`|CreateWidget` "/Game/Blueprints/Hud/W_Hint.W_Hint_C" null "Hint - First Level"))
          (`UserWidget.AddToViewport` _returnvalue_5 0))
        (:`7`
          (`self.Level7`)
          (`KismetSystemLibrary.Delay` 30.0)
          (bind _returnvalue_6 (`|CreateWidget` "/Game/Blueprints/Hud/W_Hint.W_Hint_C" null "Hint - First Level"))
          (`UserWidget.AddToViewport` _returnvalue_6 0))
        (:`8`
          (`self.Level8`)
          (`KismetSystemLibrary.Delay` 30.0)
          (bind _returnvalue_7 (`|CreateWidget` "/Game/Blueprints/Hud/W_Hint.W_Hint_C" null "Hint - First Level"))
          (`UserWidget.AddToViewport` _returnvalue_7 0))
        (:`9`
          (`self.Level9`)
          (`KismetSystemLibrary.Delay` 30.0)
          (bind _returnvalue_8 (`|CreateWidget` "/Game/Blueprints/Hud/W_Hint.W_Hint_C" null "Hint - First Level"))
          (`UserWidget.AddToViewport` _returnvalue_8 0))
        (:`10`
          (`self.Level10`)
          (`KismetSystemLibrary.Delay` 30.0)
          (bind _returnvalue_9 (`|CreateWidget` "/Game/Blueprints/Hud/W_Hint.W_Hint_C" null "Hint - First Level"))
          (`UserWidget.AddToViewport` _returnvalue_9 0))))
    (:`then_1`
      (`KismetSystemLibrary.Delay` 1.0)
      (`GameplayStatics.PlaySound2D` "/Game/Blueprints/Audio/background.background" 0.3 1.0 0.0 null null))))

(event `self.Win`
  (bind _as_a_game_instance (`self.As A Game Instance`))
  (bind _noofmoves (`self.NoOfMoves`))
  (bind _level (`/Game/Blueprints/A_GameInstance.level` _as_a_game_instance))
  (bind _levelunlocked (`/Game/Blueprints/A_GameInstance.levelUnlocked` _as_a_game_instance))
  (`GameplayStatics.PlaySound2D` "/Game/Blueprints/Audio/win.win" 1.0 1.0 0.0 null null)
  (bind _asa_pcarena_bp (cast `/Game/Blueprints/PlayerController/A_PCArenaBP` (`GameplayStatics.GetPlayerController` 0)))
  (`WidgetBlueprintLibrary.SetInputMode_UIOnlyEx` _asa_pcarena_bp null)
  (set `PlayerController.bShowMouseCursor` true _asa_pcarena_bp)
  (bind _returnvalue (`|CreateWidget` "/Game/Blueprints/Hud/W_Win.W_Win_C"))
  (`UserWidget.AddToViewport` _returnvalue 2)
  (bind _returnvalue_2 (`GameplayStatics.LoadGameFromSlot` "save1"))
  (bind _asbp_save_game (cast `/Game/Blueprints/BP_SaveGame` _returnvalue_2))
  (bind _leveltomoves (`/Game/Blueprints/BP_SaveGame.LeveltoMoves` _asbp_save_game))
  (bind _value (`BlueprintMapLibrary.Map_Find` _leveltomoves _level))
  (if (== _value 0)
    (`BlueprintMapLibrary.Map_Add` _leveltomoves _level _noofmoves :!label _label_2)
    (elif (< _noofmoves _value)
      (goto _label_2)
      (else
        _)))
  (if (== _level _levelunlocked)
    (bind _output_get (set `/Game/Blueprints/A_GameInstance.levelUnlocked` (+ _levelunlocked 1) _as_a_game_instance))
    (set `/Game/Blueprints/BP_SaveGame.levelUnlocked` (`KismetMathLibrary.Clamp` _output_get 0 10) _asbp_save_game)
    (`GameplayStatics.SaveGameToSlot` _asbp_save_game "save1")
    (else
      (`GameplayStatics.SaveGameToSlot` _asbp_save_game "save1"))))

(event `self.Loose`
  (`GameplayStatics.PlaySound2D` "/Game/Blueprints/Audio/defeat.defeat" 1.0 1.0 0.0 null null)
  (bind _asa_pcarena_bp (cast `/Game/Blueprints/PlayerController/A_PCArenaBP` (`GameplayStatics.GetPlayerController` 0)))
  (`WidgetBlueprintLibrary.SetInputMode_UIOnlyEx` _asa_pcarena_bp null)
  (set `PlayerController.bShowMouseCursor` true _asa_pcarena_bp)
  (bind _returnvalue (`|CreateWidget` "/Game/Blueprints/Hud/W_Loose.W_Loose_C"))
  (`UserWidget.AddToViewport` _returnvalue 2))

(fn `UserConstructionScript`)